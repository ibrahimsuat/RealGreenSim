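; Solar panel actor that drops onto the surface beneath it with an eased animation when spawned.
; BeginPlay traces down from the mesh, ignoring GreenAreaMaster actors, to find the landing height.
; A fast looping timer runs SpawnAnim briefly, easing the root's Z from its current height toward the hit using time accumulated in Tick over Duration.
; The trace leaves persistent debug drawing enabled.
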(event `self.ReceiveBeginPlay`
  (bind _returnvalue (`SceneComponent.K2_GetComponentLocation` (`self.mesh`)))
  (bind _outactors (`GameplayStatics.GetAllActorsOfClass` "/Game/BlankDefault/enviromentBP/GreenAreaMaster.GreenAreaMaster_C"))
  (bind _outhit (`KismetSystemLibrary.LineTraceSingle` _returnvalue (- _returnvalue (0.0 0.0 1000.0)) "TraceTypeQuery1" false _outactors "Persistent"))
  (set `self.ElapsedTime` 0.01)
  (set `self.Location` (`.Location` (`GameplayStatics.BreakHitResult` _outhit)))
  (bind _returnvalue_2 (`KismetSystemLibrary.K2_SetTimer` null "SpawnAnim" 0.001 true true))
  (`KismetSystemLibrary.Delay` 0.7)
  (`KismetSystemLibrary.K2_ClearAndInvalidateTimerHandle` _returnvalue_2))

(event `self.ReceiveTick`
  (params (DeltaSeconds :type "Float (single-precision)"))
  (set `self.ElapsedTime` (+ DeltaSeconds (`self.ElapsedTime`))))

(fn `SpawnAnim`
  (`SceneComponent.K2_SetWorldLocation` (`self.DefaultSceneRoot`) (`KismetMathLibrary.MakeVector` (.x (`self.K2_GetActorLocation`)) (.y (`self.K2_GetActorLocation`)) (`KismetMathLibrary.FInterpEaseInOut` (.z (`self.K2_GetActorLocation`)) (.z (`self.Location`)) (/ (`self.ElapsedTime`) (`self.Duration`)) 5.0)) false false))

(fn `UserConstructionScript`)